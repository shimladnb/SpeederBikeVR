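; Hover thruster component, filed with the speeder bike assets, that pushes a physics-simulated primitive away from surfaces below it using a spring-damper force.
; initComponent stores the given mesh and enables physics on it.
; Each tick it traces along its own down vector up to HoverDistance and, on a hit, applies force at its location from compression and rate of change.
; A separate TraceDown helper casts a long world-down trace, unused here.
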(event `initComponent`
  (params (meshComponent :type "StaticMeshComponent Object Reference"))
  (bind _asprimitive_component (cast `PrimitiveComponent` meshComponent))
  (set `self.parentComponent` _asprimitive_component)
  (`PrimitiveComponent.SetSimulatePhysics` (`self.parentComponent`) true)
  (set `self.validParent` (`KismetSystemLibrary.IsValid` (`self.parentComponent`))))

(event `self.ReceiveTick`
  (params (DeltaSeconds :type "Float (single-precision)"))
  (if (`self.validParent`)
    (bind (_outhit _returnvalue) (`KismetSystemLibrary.LineTraceSingle` :`Start` (`self.K2_GetComponentLocation`) :`End` (- (`self.K2_GetComponentLocation`) (* (`self.GetUpVector`) (`self.hoverDistance`))) :`TraceChannel` "TraceTypeQuery1" :`DrawDebugType` "ForOneFrame"))
    (if _returnvalue
      (bind _output_get (set `self.hoverDelta` (- (`self.hoverDistance`) (`.Distance` (`GameplayStatics.BreakHitResult` _outhit)))))
      (`PrimitiveComponent.AddForceAtLocation` (`self.parentComponent`) (* (`self.GetUpVector`) (+ (* (/ (- _output_get (`self.previousHoverDelta`)) (`GameplayStatics.GetWorldDeltaSeconds`)) (`self.dampeningCoefficient`)) (* _output_get (`self.springCoefficient`)))) (`self.K2_GetComponentLocation`) "None")
      (set `self.previousHoverDelta` (`self.hoverDelta`)))))

(fn `traceDown`
  (params (traceStart :type "Vector Structure"))
  (`KismetSystemLibrary.LineTraceSingle` :`Start` traceStart :`End` (`KismetMathLibrary.MakeVector` (.x traceStart) (.y traceStart) (- (.z traceStart) 9999999.0)) :`TraceChannel` "TraceTypeQuery1" :`DrawDebugType` "ForOneFrame"))