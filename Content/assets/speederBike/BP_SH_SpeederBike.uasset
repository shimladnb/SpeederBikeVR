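; Speeder bike that is driven and steered by two throttles on a child-actor handlebars Blueprint.
; Each tick, the averaged throttles set a forward speed that the bike mesh's physics velocity lerps toward.
; The signed, squared throttle difference becomes yaw torque on MoveCube, damped by counter-torque from its angular velocity.
; Roll is calculated the same way but never applied, as the roll event is empty.
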(event `self.ReceiveBeginPlay`
  (`self.setHandleBarsRef1`))

(event `self.ReceiveTick`
  (params (DeltaSeconds :type "Float (single-precision)"))
  (`self.setAcceleration1`)
  (`self.setRollAndSteer`)
  (`self.moveBikeForeward1`)
  (`self.bikeRoll`)
  (`self.bikeTurn`)
  (`self.compensate`))

(event `bikeRoll`)

(event `bikeTurn`
  (`PrimitiveComponent.AddTorqueInDegrees` (`self.moveCube`) (`KismetMathLibrary.VLerp` (0.0 0.0 0.0) (* (`SceneComponent.GetUpVector` (`self.mergedBike`)) (* (`self.steer`) -1.0)) 1.0) "None" true))

(event `compensate`
  (`PrimitiveComponent.AddTorqueInDegrees` (`self.moveCube`) (/ (`KismetMathLibrary.NegateVector` (`PrimitiveComponent.GetPhysicsAngularVelocityInDegrees` (`self.moveCube`) "None")) 0.5) "None" true))

(fn `moveBikeForeward1`
  (bind _mergedbike (`self.mergedBike`))
  (bind _returnvalue (`PrimitiveComponent.GetPhysicsLinearVelocity` _mergedbike "None"))
  (`PrimitiveComponent.SetPhysicsLinearVelocity` (`self.mergedBike`) (`KismetMathLibrary.VLerp` _returnvalue (* (`SceneComponent.GetForwardVector` _mergedbike) (`self.acceleration`)) 0.1) false "None"))

(fn `setAcceleration1`
  (bind _handlebarsref (`self.handleBarsRef`))
  (bind _maxspeed (`self.maxSpeed`))
  (bind _returnvalue (`KismetMathLibrary.MapRangeClamped` (`/Game/assets/speederBike/BP_SH_HandleBars.leftHandThrottle` _handlebarsref) 0.0 -60.0 0.0 _maxspeed))
  (bind _returnvalue_2 (`KismetMathLibrary.MapRangeClamped` (`/Game/assets/speederBike/BP_SH_HandleBars.rightHandThrottle` _handlebarsref) 0.0 -60.0 0.0 _maxspeed))
  (set `self.Right Hand Throttle` _returnvalue_2)
  (set `self.Left Hand Throttle` _returnvalue)
  (set `self.acceleration` (/ (+ _returnvalue_2 _returnvalue) 2.0)))

(fn `setHandleBarsRef1`
  (bind _asbp_sh_handle_bars (cast `/Game/assets/speederBike/BP_SH_HandleBars` (`ChildActorComponent.ChildActor` (`self.BP_SH_HandleBars`))))
  (set `self.handleBarsRef` _asbp_sh_handle_bars))

(fn `setRollAndSteer`
  (bind _returnvalue (/ (`self.Left Hand Throttle`) (`self.maxSpeed`)))
  (bind _returnvalue_2 (/ (`self.Right Hand Throttle`) (`self.maxSpeed`)))
  (bind _returnvalue_3 (`KismetMathLibrary.Vector_Distance2D` (`KismetMathLibrary.MakeVector` _returnvalue_2) (`KismetMathLibrary.MakeVector` _returnvalue)))
  (bind _returnvalue_4 (+ (* _returnvalue_3 (* _returnvalue_2 1.0)) (* _returnvalue_3 (* _returnvalue -1.0))))
  (set `self.roll` (* _returnvalue_4 (`self.rollMax`)))
  (set `self.steer` (* _returnvalue_4 (`self.steerMax`))))

(fn `UserConstructionScript`)