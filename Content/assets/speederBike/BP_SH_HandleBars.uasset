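; Speeder bike handlebar actor that tilts its bars and skeletal meshes to follow the VR pawn's motion controllers.
; On BeginPlay it caches the first BP_SH_SpeederBikePawn.
; Each tick, look-at pitch from the right bar's location to each controller sets that side's bar rotation and throttle value, which counter-rotates a skeletal mesh at reduced scale.
; Pickup, Drop and setHeadsetLocation are empty, and a tick counter only increments.
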(event `/Game/VirtualRealityBP/Blueprints/PickupActorInterface.Pickup`
  (params (AttachTo :type "SceneComponent Object Reference")))

(event `/Game/VirtualRealityBP/Blueprints/PickupActorInterface.Drop`)

(event `setHeadsetLocation`)

(event `self.ReceiveBeginPlay`
  (`self.setMotionControllerRef1`))

(event `self.ReceiveTick`
  (params (DeltaSeconds :type "Float (single-precision)"))
  (`self.addCounter`)
  (`self.animateBars`)
  (`self.setHeadsetLocation`))

(event `animateBars`
  (bind _returnvalue (* (.pitch (`KismetMathLibrary.FindLookAtRotation` (`SceneComponent.RelativeLocation` (`self.handleBarR`)) (.location (`SceneComponent.GetRelativeTransform` (`/Game/VirtualRealityBP/Blueprints/BP_MotionController.MotionController` (`/Game/VirtualRealityBP/Blueprints/BP_SH_SpeederBikePawn.RightController` (`self.motionControllerPawnReference`))))))) -1.0))
  (bind _returnvalue_2 (* (.pitch (`KismetMathLibrary.FindLookAtRotation` (`SceneComponent.RelativeLocation` (`self.handleBarR`)) (.location (`SceneComponent.GetRelativeTransform` (`/Game/VirtualRealityBP/Blueprints/BP_MotionController.MotionController` (`/Game/VirtualRealityBP/Blueprints/BP_SH_SpeederBikePawn.LeftController` (`self.motionControllerPawnReference`))))))) -1.0))
  (`SceneComponent.K2_SetRelativeRotation` (`self.handleBarR`) (`KismetMathLibrary.MakeRotator` 0.0 _returnvalue) false false)
  (set `self.rightHandThrottle` _returnvalue)
  (`SceneComponent.K2_SetRelativeRotation` (`self.handleBarL`) (`KismetMathLibrary.MakeRotator` 0.0 _returnvalue_2) false false)
  (set `self.leftHandThrottle` _returnvalue_2)
  (`SceneComponent.K2_SetRelativeRotation` (`self.SkeletalMesh`) (`KismetMathLibrary.MakeRotator` 0.0 (* (`self.rightHandThrottle`) -0.2)) false false)
  (`SceneComponent.K2_SetRelativeRotation` (`self.SkeletalMesh1`) (`KismetMathLibrary.MakeRotator` 0.0 (* (`self.leftHandThrottle`) -0.2)) false false))

(fn `addCounter`
  (set `self.counter` (+ (`self.counter`) 1.0)))

(fn `setMotionControllerRef1`
  (bind _outactors (`GameplayStatics.GetAllActorsOfClass` "/Game/VirtualRealityBP/Blueprints/BP_SH_SpeederBikePawn.BP_SH_SpeederBikePawn_C"))
  (set `self.motionControllerPawnReference` (`|GetArrayItem` _outactors)))

(fn `UserConstructionScript`)