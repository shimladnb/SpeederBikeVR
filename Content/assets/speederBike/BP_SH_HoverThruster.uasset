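; Hover thruster component for the speeder bike that pushes a physics-simulated primitive away from the surface beneath it.
; Its init event stores the supplied mesh and enables physics simulation on it.
; Each tick it traces along its local down axis and applies force at its own location along the hit normal, fading linearly to zero at full trace length.
; A separate TraceDown helper does a long world-down trace but is not called here.
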(event `initComponent`
  (params (meshComponent :type "StaticMeshComponent Object Reference"))
  (bind _asprimitive_component (cast `PrimitiveComponent` meshComponent))
  (set `self.parentComponent` _asprimitive_component)
  (`PrimitiveComponent.SetSimulatePhysics` (`self.parentComponent`) true))

(event `self.ReceiveTick`
  (params (DeltaSeconds :type "Float (single-precision)"))
  (bind _returnvalue (`self.K2_GetComponentLocation`))
  (bind (_outhit _returnvalue_2) (`KismetSystemLibrary.LineTraceSingle` :`Start` _returnvalue :`End` (+ _returnvalue (* (* (`self.GetUpVector`) -1.0) (`self.traceLength`))) :`TraceChannel` "TraceTypeQuery1" :`DrawDebugType` "ForOneFrame"))
  (if _returnvalue_2
    (bind (_bblockinghit _binitialoverlap _time _distance _location _impactpoint _normal _impactnormal) (`GameplayStatics.BreakHitResult` _outhit))
    (`PrimitiveComponent.AddForceAtLocation` (`self.parentComponent`) (* _impactnormal (`KismetMathLibrary.Lerp` (* (`self.hoverForce`) 100000.0) 0.0 (/ (`KismetMathLibrary.VSize` (- _location (`self.K2_GetComponentLocation`))) (`self.traceLength`)))) (`self.K2_GetComponentLocation`) "None")))

(fn `traceDown`
  (params (traceStart :type "Vector Structure"))
  (`KismetSystemLibrary.LineTraceSingle` :`Start` traceStart :`End` (`KismetMathLibrary.MakeVector` (.x traceStart) (.y traceStart) (- (.z traceStart) 9999999.0)) :`TraceChannel` "TraceTypeQuery1" :`DrawDebugType` "ForOneFrame"))